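; BP_Cannon is a cannon actor that automatically fires a cannonball about once per second from BeginPlay onward.
; BeginPlay loops through a one-second Delay into the FireCannon event.
; FireCannon prints the shot count, spawns a BP_Cannonball at SpawnPoint's transform, and increments the count.
; It launches each ball's Cube with a single mass-independent AddForce along SpawnPoint's forward vector.
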(event `self.ReceiveBeginPlay`
  (`KismetSystemLibrary.Delay` 1.0 :!label _label)
  (`self.FireCannon`)
  (goto _label))

(event `FireCannon`
  (`KismetSystemLibrary.PrintText` (`|FormatText` "Firing the {count}th cannonball!" (`self.ShotCount`)) true true (struct :`G` 0.66 :`B` 1.0 :`A` 1.0) 0.1)
  (bind _returnvalue (`|SpawnActorFromClass` "/Game/Blueprints/BP_Cannonball.BP_Cannonball_C" (`SceneComponent.K2_GetComponentToWorld` (`self.SpawnPoint`)) "Undefined" "MultiplyWithRoot" null null)) ; Spawn Actor From Class
  (`PrimitiveComponent.AddForce` (`/Game/Blueprints/BP_Cannonball.Cube` _returnvalue) (* (`SceneComponent.GetForwardVector` (`self.SpawnPoint`)) 1000000.0) "None" true)
  (`/Engine/EditorBlueprintResources/StandardMacros.IncrementInt` (`self.ShotCount`)))

(fn `UserConstructionScript`)
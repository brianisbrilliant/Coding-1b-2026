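; Dialogue manager Blueprint that shows lines from a Dialogue string array one at a time, each time DisplayNextLine fires.
; BeginPlay creates and caches a W_Dialogue widget; each line sets its text, also prints for debugging, and appears in the viewport for five seconds.
; A Sequence increments Index without waiting for that delay.
; Past the last line, ShouldRepeatText either restarts from the first or shows nothing.
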(event `self.ReceiveBeginPlay`
  (bind _returnvalue (`|CreateWidget` "/Game/Widgets/W_Dialogue.W_Dialogue_C")) ; "create widget"
  (set `self.Dialogue Widget` _returnvalue) ; Promote to Variable
)

(event `DisplayNextLine`
  (bind _dialogue_widget (`self.Dialogue Widget`))
  (bind _output (`|GetArrayItem` (`self.Dialogue`) (`self.index`)))
  (if (>= (`self.index`) (`KismetArrayLibrary.Array_Length` (`self.Dialogue`)))
    (if (`self.ShouldRepeatText`)
      (set `self.index` 0)
      (`KismetSystemLibrary.PrintText` _output true true (struct :`R` 1.0 :`G` 0.445856 :`A` 1.0) 5.0 :!label _label)
      (`TextBlock.SetText` (`/Game/Widgets/W_Dialogue.TextBlock_0` (`self.Dialogue Widget`)) _output)
      (`|ExecutionSequence`
        (:`then_0`
          (`UserWidget.AddToViewport` _dialogue_widget 0) ; add the dialogue to the view
          (`KismetSystemLibrary.Delay` 5.0) ; wait 5 seconds
          (`Widget.RemoveFromParent` _dialogue_widget) ; remove the dialogue from the view
        )
        (:`then_1`
          (`/Engine/EditorBlueprintResources/StandardMacros.IncrementInt` (`self.index`)) ; Increment Int\nto add 1 to our index
        )))
    (else
      (goto _label))))

(fn `UserConstructionScript`)
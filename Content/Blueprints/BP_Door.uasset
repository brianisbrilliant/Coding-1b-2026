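; BP_Door is a locked door actor that opens when the player character touches it while holding a key.
; On overlap it casts to BP_ThirdPersonCharacter_old and reads that character's TotalKeys count.
; With a key, it spends one and destroys its door mesh and box collision components; otherwise it prints a locked message.
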(event `self.ReceiveActorBeginOverlap`
  (params (OtherActor :type "Actor Object Reference"))
  (bind _asbp_third_person_character (cast `/Game/ThirdPerson/Blueprints/BP_ThirdPersonCharacter_old` OtherActor))
  (`KismetSystemLibrary.PrintText` "ThePlayer is knocking!")
  (bind _totalkeys (`/Game/ThirdPerson/Blueprints/BP_ThirdPersonCharacter_old.TotalKeys` _asbp_third_person_character))
  (if (> _totalkeys 0)
    (`/Engine/EditorBlueprintResources/StandardMacros.DecrementInt` _totalkeys ; remove a key\nfrom totalKeys
      (:`  `
        (`ActorComponent.K2_DestroyComponent` (`self.SM_Bld_Door_01`))
        (`ActorComponent.K2_DestroyComponent` (`self.BoxCollision`))))
    (else
      (`KismetSystemLibrary.PrintText` "I am locked!"))))

(fn `UserConstructionScript`)
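; BP_LoopsAndLists is a demo Blueprint of loop and array techniques, using printed text and BP_Tree actors.
; BeginPlay starts an endless three-second Delay loop and a while loop that prints a countdown in cycling colors.
; Each three-second pass calls LoopArrayOverTime, which shuffles the trees and randomizes their yaw at 0.2-second intervals through a Delay-driven index loop.
; ChangeTreesForEach rotates every tree at once, but nothing here calls it.
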(event `self.ReceiveBeginPlay`
  (`KismetSystemLibrary.PrintText` "Loops and Lists is Starting")
  (`self.Simple Loop`)
  (`self.WhileLoop Function`))

(event `Simple Loop`
  (`KismetSystemLibrary.PrintText` "Inside Simple Loop, waiting 3 seconds." :!label _label)
  (`self.LoopArrayOverTime`)
  (`KismetSystemLibrary.Delay` 3.0)
  (goto _label))

(event `WhileLoop Function`
  (bind _colors (`self.Colors`))
  (while (> (`self.WhileCounter`) 0)
    (`KismetSystemLibrary.PrintText` (`|FormatText` "This is loop {count}. Ran after {seconds} seconds." (`self.WhileCounter`) (`KismetTextLibrary.Conv_DoubleToText` (`GameplayStatics.GetRealTimeSeconds`) "HalfToEven" false true 1 324 3)) true true (`|GetArrayItem` _colors (mod (`self.WhileCounter`) (`KismetArrayLibrary.Array_Length` _colors))) 20.0)
    (`/Engine/EditorBlueprintResources/StandardMacros.DecrementInt` (`self.WhileCounter`)) ; decrement int
  ))

(event `ChangeTreesForEach`
  (bind _outactors (`GameplayStatics.GetAllActorsOfClass` "/Game/Blueprints/BP_Tree.BP_Tree_C"))
  (for _array_element _outactors
    (`self.K2_SetActorRelativeRotation` _array_element (`KismetMathLibrary.MakeRotator` 0.0 0.0 (`KismetMathLibrary.RandomFloatInRange` 0.0 360.0)) false false))
  (`KismetSystemLibrary.PrintText` "Trees have been rotated."))

(event `LoopArrayOverTime`
  (bind _outactors (`GameplayStatics.GetAllActorsOfClass` "/Game/Blueprints/BP_Tree.BP_Tree_C"))
  (`KismetArrayLibrary.Array_Shuffle` _outactors)
  (if (< (`self.OverTimeIndex`) (`KismetArrayLibrary.Array_Length` _outactors)) :!label _label_2
    (`self.K2_SetActorRelativeRotation` (`|GetArrayItem` _outactors (`self.OverTimeIndex`)) (`KismetMathLibrary.MakeRotator` 0.0 0.0 (`KismetMathLibrary.RandomFloatInRange` 0.0 360.0)) false false)
    (`/Engine/EditorBlueprintResources/StandardMacros.IncrementInt` (`self.OverTimeIndex`) ; Increment int
      (:`  `
        (`KismetSystemLibrary.Delay` 0.2)
        (goto _label_2)))
    (else
      (set `self.OverTimeIndex` 0) ; reset index to zero, so we can \nloop again
    )))

(fn `UserConstructionScript`)
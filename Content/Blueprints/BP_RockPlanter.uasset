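; BP_RockPlanter is a pickup item that a third-person character can carry and use to plant objects.
; Overlap stores the character and calls its TryToPickupItem, while the Pickup event snaps the item to the hand grip socket.
; PrimaryAction spawns BP_Tree at the planter's transform, despite the rock naming, with floor line-trace placement still a TODO.
; Drop destroys the planter instead of releasing it.
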(event `self.ReceiveActorBeginOverlap`
  (params (OtherActor :type "Actor Object Reference"))
  (bind _asbp_third_person_character (cast `/Game/ThirdPerson/Blueprints/BP_ThirdPersonCharacter` OtherActor))
  (set `self.Player` _asbp_third_person_character) ; Promote To Variable
  (`/Game/ThirdPerson/Blueprints/BP_ThirdPersonCharacter.TryToPickupItem` _asbp_third_person_character self))

(event `/Game/Blueprints/BPI_Item.Pickup`
  (`KismetSystemLibrary.PrintText` "The Rock Planter is getting picked up!")
  (`self.K2_AttachToComponent` (`Character.Mesh` (`self.Player`)) "HandGrip_R" "SnapToTarget" "SnapToTarget" "KeepRelative"))

(event `/Game/Blueprints/BPI_Item.PrimaryAction`
  (`KismetSystemLibrary.PrintText` "Let's plant some rocks!")
  ; TODO: Use a linetrace to spawn rock on floor
  (`|SpawnActorFromClass` "/Game/Blueprints/BP_Tree.BP_Tree_C" (`self.GetTransform`) "Undefined" "MultiplyWithRoot" null null))

(event `/Game/Blueprints/BPI_Item.Drop`
  (`KismetSystemLibrary.PrintText` "The Rock Planter is getting Dropped!")
  (`self.K2_DestroyActor`))

(fn `UserConstructionScript`)